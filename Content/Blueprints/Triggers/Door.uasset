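; Door trigger Blueprint that slides a door open once the player character has collected enough statues.
; On Enter, it casts the player pawn to ThirdPersonCharacter and compares its Statues count with StatuesToOpen.
; When the count is met, DoorTimeline plays and drives the Mesh relative location from its Sliding track.
; Exit reverses the timeline to slide the door back.
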(event `self.Enter`
  (bind _asthird_person_character (cast `/Game/ThirdPersonBP/Blueprints/ThirdPersonCharacter` (`GameplayStatics.GetPlayerCharacter` 0)))
  (if (>= (`/Game/ThirdPersonBP/Blueprints/ThirdPersonCharacter.Statues` _asthird_person_character) (`self.StatuesToOpen`))
    (bind (_direction _sliding) (`Timeline|DoorTimeline` :!label _label)
      (:`Update`
        (`SceneComponent.K2_SetRelativeLocation` (`self.Mesh`) _sliding false false)))))

(event `self.Exit`
  (goto _label :!via `Reverse`))

(fn `UserConstructionScript`
  (`parent.UserConstructionScript`))